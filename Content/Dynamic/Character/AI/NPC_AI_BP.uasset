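; NPC AI controller that runs a guard behavior tree and reacts to perceived actors.
; On BeginPlay it sets up the patrol blackboard and starts the tree.
; Perception updates for actors without the "Enemy" tag store the sensed actor as the enemy key, or clear it when sensing fails.
; The same updates switch the controlled character's aiming and shooting flags on or off.
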(event `self.ReceiveBeginPlay`
  (bind _blackboardcomponent (`self.UseBlackboard` "/Game/Dynamic/Character/AI/PatrolData.PatrolData"))
  (`self.RunBehaviorTree` "/Game/Dynamic/Character/AI/GuardBehaviour.GuardBehaviour")
  (set `self.Blackboard Component` _blackboardcomponent))

(event `self.AIPerception.OnTargetPerceptionUpdated`
  (params (Actor :type "Actor Object Reference") (Stimulus :type "AIStimulus Structure"))
  (bind _returnvalue (`self.K2_GetPawn`))
  (bind _blackboard_component (`self.Blackboard Component`))
  (bind _enemykey (`self.EnemyKey`))
  (if (`self.ActorHasTag` Actor "Enemy")
    _
    (elif (`.bSuccessfullySensed` (break `AIStimulus` Stimulus))
      (`BlackboardComponent.SetValueAsObject` _blackboard_component _enemykey Actor)
      (bind _astp_character (cast `/Game/Dynamic/Character/Behaviour/Character` _returnvalue))
      (set `/Game/Dynamic/Character/Behaviour/Character.Aiming` true _astp_character)
      (set `/Game/Dynamic/Character/Behaviour/Character.Shooting` true _astp_character)
      (else
        (`BlackboardComponent.ClearValue` _blackboard_component _enemykey)
        (bind _astp_character_2 (cast `/Game/Dynamic/Character/Behaviour/Character` _returnvalue))
        (set `/Game/Dynamic/Character/Behaviour/Character.Aiming` false _astp_character_2)
        (set `/Game/Dynamic/Character/Behaviour/Character.Shooting` false _astp_character_2)))))

(fn `UserConstructionScript`)