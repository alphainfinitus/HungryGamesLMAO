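; An AI controller for guard NPCs that runs a guard behavior tree and reacts to perceived targets.
; On BeginPlay it sets up the PatrolData blackboard and starts GuardBehaviour.
; AI Perception updates for actors not tagged "Enemy" write the sensed actor to the enemy blackboard key, or clear it when sensing is lost.
; The same updates toggle the controlled character's Aiming flag.
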(event `self.ReceiveBeginPlay`
  (bind _blackboardcomponent (`self.UseBlackboard` "/Game/Dynamic/NPC/AI/PatrolData.PatrolData"))
  (`self.RunBehaviorTree` "/Game/Dynamic/NPC/AI/GuardBehaviour.GuardBehaviour")
  (set `self.Blackboard Component` _blackboardcomponent))

(event `self.AIPerception.OnTargetPerceptionUpdated`
  (params (Actor :type "Actor Object Reference") (Stimulus :type "AIStimulus Structure"))
  (bind _returnvalue (`self.K2_GetPawn`))
  (bind _blackboard_component (`self.Blackboard Component`))
  (bind _enemykey (`self.EnemyKey`))
  (if (`self.ActorHasTag` Actor "Enemy")
    _
    (elif (`.bSuccessfullySensed` (break `AIStimulus` Stimulus))
      (`BlackboardComponent.SetValueAsObject` _blackboard_component _enemykey Actor)
      (bind _asue_4asp_character (cast `/Game/Dynamic/NPC/Behaviour/Ue4ASP_Character` _returnvalue))
      (set `/Game/Dynamic/NPC/Behaviour/Ue4ASP_Character.Aiming` true _asue_4asp_character)
      (else
        (`BlackboardComponent.ClearValue` _blackboard_component _enemykey)
        (bind _asue_4asp_character_2 (cast `/Game/Dynamic/NPC/Behaviour/Ue4ASP_Character` _returnvalue))
        (set `/Game/Dynamic/NPC/Behaviour/Ue4ASP_Character.Aiming` false _asue_4asp_character_2)))))

(fn `UserConstructionScript`)