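; Terrain tile for an infinite terrain mode that fills itself with random numbers of props and rocks on BeginPlay via PlaceActors.
; Its barrier wall starts solid and opaque, turning passable and transparent while the player overlaps the locking volume.
; Leaving that volume relocks the wall and asks InfiniteTerrainGameMode to spawn a tile.
; The tile exposes its Arrow transform as an attach point and destroys itself when the player enters the destroying volume.
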(event `self.ReceiveBeginPlay`
  (`self.LockBarrier`)
  (`self.PlaceActors` "/Game/Dynamic/Terrain/Props/BP_Container.BP_Container_C" 1 3)
  (`self.PlaceActors` "/Game/Dynamic/Terrain/Props/BP_Box.BP_Box_C" 2 4)
  (`self.PlaceActors` "/Game/Dynamic/Terrain/Props/BP_Canister.BP_Canister_C" 3 7)
  (`self.PlaceActors` "/Game/Dynamic/Terrain/Props/BP_Rock1.BP_Rock1_C" 0 3)
  (`self.PlaceActors` "/Game/Dynamic/Terrain/Props/BP_Rock17.BP_Rock17_C" 0 3)
  (`self.PlaceActors` "/Game/Dynamic/Terrain/Props/BP_Rocks.BP_Rocks_C" 0 3)
  (`self.PlaceActors` "/Game/Dynamic/Terrain/Props/BP_SackLine.BP_SackLine_C" 0 3)
  (`self.PlaceActors` "/Game/Dynamic/Terrain/Props/BP_Rock5.BP_Rock5_C" 0 3))

(event `self.Locking Volume.OnComponentBeginOverlap`
  (params (OverlappedComponent :type "PrimitiveComponent Object Reference") (OtherActor :type "Actor Object Reference") (OtherComp :type "PrimitiveComponent Object Reference") (OtherBodyIndex :type Integer) (bFromSweep :type Boolean) (SweepResult :type "HitResult Structure (by ref)"))
  (`self.IsPlayerActor` OtherActor)
  (`self.UnlockBarrier`))

(event `self.Locking Volume.OnComponentEndOverlap`
  (params (OverlappedComponent :type "PrimitiveComponent Object Reference") (OtherActor :type "Actor Object Reference") (OtherComp :type "PrimitiveComponent Object Reference") (OtherBodyIndex :type Integer))
  (`self.IsPlayerActor` OtherActor)
  (`self.LockBarrier`)
  (bind _asinfinite_terrain_game_mode (cast `/Game/Dynamic/InfiniteTerrainGameMode` (`GameplayStatics.GetGameMode`)))
  (`/Game/Dynamic/InfiniteTerrainGameMode.SpawnTile` _asinfinite_terrain_game_mode))

(event `self.Destroying Volume.OnComponentBeginOverlap`
  (params (OverlappedComponent :type "PrimitiveComponent Object Reference") (OtherActor :type "Actor Object Reference") (OtherComp :type "PrimitiveComponent Object Reference") (OtherBodyIndex :type Integer) (bFromSweep :type Boolean) (SweepResult :type "HitResult Structure (by ref)"))
  (`self.IsPlayerActor` OtherActor)
  (`self.K2_DestroyActor`))

(fn `GetAttachLocation`
  (returns (`Attach Transform` :type "Transform Structure"))
  (return (`SceneComponent.K2_GetComponentToWorld` (`self.Arrow`))))

(fn `LockBarrier`
  (`PrimitiveComponent.SetCollisionEnabled` (`self.Barrier Wall`) "QueryAndPhysics")
  (`PrimitiveComponent.SetMaterial` (`self.Barrier Wall`) 0 "/Game/Dynamic/Terrain/MI_Barrier_Opaque.MI_Barrier_Opaque"))

(fn `UnlockBarrier`
  (`PrimitiveComponent.SetCollisionEnabled` (`self.Barrier Wall`) "NoCollision")
  (`PrimitiveComponent.SetMaterial` (`self.Barrier Wall`) 0 "/Game/Dynamic/Terrain/MI_Barrier_Transparent.MI_Barrier_Transparent"))

(fn `UserConstructionScript`)