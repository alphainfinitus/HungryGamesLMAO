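; Terrain tile actor for an infinite terrain system, with a barrier wall that opens for the player and tiles that spawn and destroy as they advance.
; Entering LockingVolume makes the barrier transparent and passable; leaving restores it and asks InfiniteTerrainGameMode to spawn another tile.
; Player overlap with DestroyingVolume destroys the tile.
; GetAttachLocation exposes the Arrow's world transform as an attach point.
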(event `self.ReceiveBeginPlay`
  (`self.LockBarrier`))

(event `self.Locking Volume.OnComponentBeginOverlap`
  (params (OverlappedComponent :type "PrimitiveComponent Object Reference") (OtherActor :type "Actor Object Reference") (OtherComp :type "PrimitiveComponent Object Reference") (OtherBodyIndex :type Integer) (bFromSweep :type Boolean) (SweepResult :type "HitResult Structure (by ref)"))
  (`self.IsPlayerActor` OtherActor)
  (`self.UnlockBarrier`))

(event `self.Locking Volume.OnComponentEndOverlap`
  (params (OverlappedComponent :type "PrimitiveComponent Object Reference") (OtherActor :type "Actor Object Reference") (OtherComp :type "PrimitiveComponent Object Reference") (OtherBodyIndex :type Integer))
  (`self.IsPlayerActor` OtherActor)
  (`self.LockBarrier`)
  (bind _asinfinite_terrain_game_mode (cast `/Game/Dynamic/InfiniteTerrainGameMode` (`GameplayStatics.GetGameMode`)))
  (`/Game/Dynamic/InfiniteTerrainGameMode.SpawnTile` _asinfinite_terrain_game_mode))

(event `self.Destroying Volume.OnComponentBeginOverlap`
  (params (OverlappedComponent :type "PrimitiveComponent Object Reference") (OtherActor :type "Actor Object Reference") (OtherComp :type "PrimitiveComponent Object Reference") (OtherBodyIndex :type Integer) (bFromSweep :type Boolean) (SweepResult :type "HitResult Structure (by ref)"))
  (`self.IsPlayerActor` OtherActor)
  (`self.K2_DestroyActor`))

(fn `GetAttachLocation`
  (returns (`Attach Transform` :type "Transform Structure"))
  (return (`SceneComponent.K2_GetComponentToWorld` (`self.Arrow`))))

(fn `LockBarrier`
  (`PrimitiveComponent.SetCollisionEnabled` (`self.Barrier Wall`) "QueryAndPhysics")
  (`PrimitiveComponent.SetMaterial` (`self.Barrier Wall`) 0 "/Game/Dynamic/Terrain/OpaqueBarrier.OpaqueBarrier"))

(fn `UnlockBarrier`
  (`PrimitiveComponent.SetCollisionEnabled` (`self.Barrier Wall`) "NoCollision")
  (`PrimitiveComponent.SetMaterial` (`self.Barrier Wall`) 0 "/Game/Dynamic/Terrain/TransparentBarrier.TransparentBarrier"))

(fn `UserConstructionScript`)